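; NewPawn is a test pawn for damage handling that also adds a NewWidgetBlueprint widget to the viewport on BeginPlay.
; Pressing M applies damage to the pawn itself, which triggers AnyDamage.
; That handler sets Health straight to zero and always prints "dead", as its branch condition is hardcoded true.
; The subtraction and below-zero check nodes are left unconnected, so the damage amount is ignored.
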(event Collision|EventActorBeginOverlap
  (params (OtherActor :type Actor%20Object%20Reference)))

(event EventTick
  (params (DeltaSeconds :type Float%20%28single-precision%29)))

(event Game|Damage|EventAnyDamage
  (params (Damage :type Float%20%28single-precision%29) (DamageType :type Damage%20Type%20Object%20Reference) (InstigatedBy :type Controller%20Object%20Reference) (DamageCauser :type Actor%20Object%20Reference))
  (Variables|Default|Sethealth 0.0)
  (if true
    (Development|PrintString "dead")
    (else
      (Development|PrintString (Utilities|String|ToString(Float) (Variables|Default|Gethealth))))))

(event EventBeginPlay
  (bind _returnvalue (UserInterface|CreateWidget "/Game/widget/NewWidgetBlueprint.NewWidgetBlueprint_C" (Game|GetPlayerController 0)))
  (UserInterface|Viewport|AddtoViewport _returnvalue 0))

(event Input|KeyboardEvents|M
  (params (Key :type Key%20Structure :default "None"))
  (:Pressed
    (Game|Damage|ApplyDamage self 1e+01 0 0)))

(fn ConstructionScript)