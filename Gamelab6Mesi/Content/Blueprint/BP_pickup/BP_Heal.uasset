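; BP_Heal is a pickup that restores health to the player when collected.
; On pickup it casts player 0's character to BP_Character and adds Heal to its Health, capped at MaxHP.
; It then broadcasts the character's OnPlayerDamage dispatcher with the new health, reusing the damage event for healing, and hands off to the parent's OnPickup.
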(event EventOnPickup
  (bind _asbp_character (Utilities|Casting|CastToBP_Character (Game|GetPlayerCharacter 0)))
  (if (>= (+ (Variables|/Game/Blueprint/Player/BP_Character.BP_Character_C|GetHealth _asbp_character) (Variables|Default|GetHeal)) (Variables|/Game/Blueprint/Player/BP_Character.BP_Character_C|GetMaxHP _asbp_character))
    (Variables|/Game/Blueprint/Player/BP_Character.BP_Character_C|SetHealth _asbp_character (Variables|/Game/Blueprint/Player/BP_Character.BP_Character_C|GetMaxHP _asbp_character))
    (else
      (Variables|/Game/Blueprint/Player/BP_Character.BP_Character_C|SetHealth _asbp_character (+ (Variables|/Game/Blueprint/Player/BP_Character.BP_Character_C|GetHealth _asbp_character) (Variables|Default|GetHeal)))))
  (Default|CallOnPlayerDamage _asbp_character (Variables|/Game/Blueprint/Player/BP_Character.BP_Character_C|GetHealth _asbp_character))
  (|CallParentFunction))

(fn ConstructionScript
  (|CallParentFunction))