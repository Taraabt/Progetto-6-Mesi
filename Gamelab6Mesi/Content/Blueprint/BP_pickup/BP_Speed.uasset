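; BP_Speed is a pickup that temporarily changes the player character's movement speed, deriving from a parent pickup Blueprint.
; On pickup, it sets player 0's BP_Character max walk speed to MaxSpeed and destroys its Niagara component.
; After a Duration delay, it restores the character's own Speed value.
; The parent OnPickup runs only after that delay, and never if the cast fails.
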(event EventOnPickup
  (bind _asbp_character (Utilities|Casting|CastToBP_Character (Game|GetPlayerCharacter 0)))
  (Variables|/Script/Engine.CharacterMovementComponent|SetMaxWalkSpeed (Variables|/Script/Engine.Character|GetCharacterMovement _asbp_character) (Variables|Default|GetMaxSpeed))
  (Components|DestroyComponent (Variables|Default|GetNiagara))
  (Utilities|FlowControl|Delay (Variables|Default|GetDuration))
  (Variables|/Script/Engine.CharacterMovementComponent|SetMaxWalkSpeed (Variables|/Script/Engine.Character|GetCharacterMovement _asbp_character) (Variables|/Game/Blueprint/Player/BP_Character.BP_Character_C|GetSpeed _asbp_character))
  (|CallParentFunction))

(fn ConstructionScript
  (|CallParentFunction))