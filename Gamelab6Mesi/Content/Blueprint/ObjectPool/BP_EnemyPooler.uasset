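; Enemy pool manager Blueprint that pre-creates enemies and tracks their deaths against spawner progress.
; On BeginPlay, it initializes the pool through BPEnemyPoolerComponent, then binds an event to the death of each pooled BP_EnemyAI.
; Its OnEnemyDeath handler raises the indexed spawner's Perc by a fixed step and decrements EnemyToKill.
; The check on remaining kills leads to no further action.
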(event Custom|OnEnemyDeath
  (bind _spawner (Variables|Default|GetSpawner))
  (bind _index (Variables|Default|GetIndex))
  (bind _output (Utilities|Array|Get(acopy) _spawner _index))
  (Variables|/Game/Blueprint/Enemy/BP_EnemySpawner.BP_EnemySpawner_C|SetPerc _output (+ (Variables|/Game/Blueprint/Enemy/BP_EnemySpawner.BP_EnemySpawner_C|GetPerc _output) 1e+01))
  (bind _result (Math|Integer|DecrementInt (Variables|/Game/Blueprint/Enemy/BP_EnemySpawner.BP_EnemySpawner_C|GetEnemyToKill _output))
    (:%20%20
      (if (> _result 0)
        _))))

(event EventBeginPlay
  (Default|InitializePool (Variables|Default|GetBP_EnemyPoolerComponent))
  (CallFunction|BindingEvent))

(fn ConstructionScript)

(fn BindingEvent
  (for _array_element (Variables|/Game/Blueprint/ObjectPool/BP_EnemyPoolerComponent.BP_EnemyPoolerComponent_C|GetObjectPool (Variables|Default|GetBP_EnemyPoolerComponent))
    (bind _asbp_enemy_ai (Utilities|Casting|CastToBP_EnemyAI _array_element))
    (EventDispatchers|BindEventtoOnDeath _asbp_enemy_ai (EventDispatchers|CreateEvent :!event Custom|OnEnemyDeath))))