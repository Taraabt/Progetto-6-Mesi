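; Actor component that pre-spawns and reuses pooled actors, apparently enemies, for several classes.
; InitializePool decrements PoolSize, then fills one flat ObjectPool with a batch per class, marking each actor not in use.
; SpawnFromPool takes a class index, searches a range offset by the decremented PoolSize for a free actor, then moves and activates it.
; It prints "Failed" when none is free, without growing the pool.
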(event Custom|InitializePool
  (bind _poolsize (Variables|Default|GetPoolSize))
  (Math|Integer|DecrementInt _poolsize
    (:%20%20
      (for _array_element (Variables|Default|GetPooledObjectClass)
        (for _index (range 0 _poolsize)
          (bind _returnvalue (Game|SpawnActorfromClass _array_element (Math|Transform|MakeTransform "0, 0, 0" "0, 0, 0" "1.000000,1.000000,1.000000") "Undefined" "MultiplyWithRoot" 0 0))
          (Utilities|Array|AddUnique (Variables|Default|GetObjectPool) _returnvalue)
          (Default|SetinUse _returnvalue false))))))

(event EventTick
  (params (DeltaSeconds :type Float%20%28single-precision%29)))

(fn FindFirstObject
  (params (Index :type Integer))
  (bind _poolsize (Variables|Default|GetPoolSize))
  (bind _output_get (Variables|Default|SetIndex Index))
  (for _index (range (* _output_get _poolsize) (+ (* _output_get _poolsize) (- _poolsize 1)))
    (if (not (Variables|/Game/Blueprint/ObjectPool/BP_PooledObject.BP_PooledObject_C|GetInUse (Utilities|Array|Get(acopy) (Variables|Default|GetObjectPool) _index)))
      (return (Utilities|Array|Get(acopy) (Variables|Default|GetObjectPool) _index)))))

(fn SpawnfromPool
  (params (SpawnTransform :type Transform) (Index :type Integer))
  (bind _pooledobject (CallFunction|FindFirstObject Index))
  (Utilities|IsValid _pooledobject
    (:Is%20Valid
      (Transformation|SetActorTransform _pooledobject SpawnTransform)
      (Default|SetinUse _pooledobject true)
      (return _pooledobject))
    (:Is%20Not%20Valid
      (Development|PrintString "Failed"))))