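; BP_ObjectPooler is an object pool actor that pre-spawns actors of a configurable class for reuse.
; On BeginPlay it fills the ObjectPool array in a loop driven by PoolSize, marking each actor as not in use.
; SpawnFromPool linearly searches for the first free actor, moves it to the given transform and marks it in use.
; The pool never grows, so a request with no free actor only prints a failure message.
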(event Custom|InitializePool
  (for _index (range 0 (Variables|Default|GetPoolSize))
    (bind _returnvalue (Game|SpawnActorfromClass (Variables|Default|GetPooledObjectClass) (Math|Transform|MakeTransform "0, 0, 0" "0, 0, 0" "1.000000,1.000000,1.000000") "Undefined" "MultiplyWithRoot" 0 0))
    (Utilities|Array|AddUnique (Variables|Default|GetObjectPool) _returnvalue)
    (Default|SetinUse _returnvalue false)))

(event EventBeginPlay
  (CallFunction|InitializePool))

(event EventTick
  (params (DeltaSeconds :type Float%20%28single-precision%29)))

(fn FindFirstObject
  (for _array_element (Variables|Default|GetObjectPool)
    (if (not (Variables|/Game/Blueprint/ObjectPool/BP_PooledObject.BP_PooledObject_C|GetInUse _array_element))
      (return _array_element))))

(fn SpawnfromPool
  (params (SpawnTransform :type Transform))
  (bind _pooledobject (CallFunction|FindFirstObject))
  (Utilities|IsValid _pooledobject
    (:Is%20Valid
      (Transformation|SetActorTransform _pooledobject SpawnTransform)
      (Default|SetinUse _pooledobject true)
      (return _pooledobject))
    (:Is%20Not%20Valid
      (Development|PrintString "Failed"))))