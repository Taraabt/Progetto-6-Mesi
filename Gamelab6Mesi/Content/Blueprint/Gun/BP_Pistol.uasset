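; BP_Pistol is a gun Blueprint that fires projectiles for the player's BP_Character and tracks its own ammo.
; Shoot uses the CanShoot macro to check the character's reload and want-shoot state, spends a round, reports the count, then spawns the projectile, muzzle effect and sound at the Arrow.
; A Timeline drives recoil by lerping the skeletal mesh toward RecoilPosition, scaled by RecoilIntensity.
; Shooting while empty triggers the character's Reload.
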(event EventBeginPlay
  (|CallParentFunction)
  (bind _output_get (Variables|Default|SetMaxAmmo (Variables|Default|GetPistolMaxAmmo)))
  (Variables|Default|SetAmmo _output_get)
  (bind _asbp_character (Utilities|Casting|CastToBP_Character (Game|Player|GetPlayerPawn 0)))
  (Default|CallOnAmmoChanged _asbp_character _output_get))

(event EventShoot
  (bind _arrow (Variables|Default|GetArrow))
  (bind _ammo (Variables|Default|GetAmmo))
  (bind _returnvalue (Transformation|GetRelativeTransform _arrow))
  (bind (_location _rotation) (Math|Transform|BreakTransform _returnvalue))
  (if (> (Variables|Default|GetAmmo) 0)
    (Utilities|CanShoot
      (:true
        (Math|Integer|DecrementInt _ammo
          (:%20%20
            (bind _asbp_character (Utilities|Casting|CastToBP_Character (Game|GetPlayerCharacter 0)))
            (Default|CallOnAmmoChanged _asbp_character _ammo)
            (Utilities|FlowControl|Sequence
              (:then_0
                (Game|SpawnActorfromClass "/Game/Blueprint/Projectile/BP_PistolProjectile.BP_PistolProjectile_C" (Transformation|GetWorldTransform _arrow) "AlwaysSpawn" "MultiplyWithRoot" 0 0)
                (Effects|SpawnEmitterAttached "/Game/Unreal/StarterContent/Particles/P_Explosion.P_Explosion" (Variables|Default|GetArrow) "None" _location _rotation "0.200000,0.200000,0.200000")
                (Audio|PlaySoundatLocation "/Game/Unreal/StarterContent/Audio/Collapse_Cue.Collapse_Cue" (Transformation|GetWorldLocation (Variables|Default|GetArrow)) "0, 0, 0" 0.1 1.0 0.0 0 0 0 0))
              (:then_1
                (bind _newtrack_0 (Timeline|Timeline PlayFromStart)
                  (:Update
                    (Transformation|SetRelativeTransform (Variables|Default|GetSkeletalMesh) (Math|Transform|Lerp(Transform) (Math|Transform|MakeTransform "-5.000000,0.000000,1.000000" "0.000000,180.000000,0.000000" "5.000000,5.000000,5.000000") (Variables|Default|GetRecoil%20Position) (* _newtrack_0 (Variables|Default|GetRecoil%20Intensity))) false false)))))))))
    (else
      (bind _asbp_character_2 (Utilities|Casting|CastToBP_Character (Game|GetPlayerCharacter 0)))
      (Default|Reload _asbp_character_2))))

(fn ConstructionScript
  (|CallParentFunction))