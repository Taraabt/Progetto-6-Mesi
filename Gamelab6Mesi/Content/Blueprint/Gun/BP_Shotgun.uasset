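; Shotgun weapon, derived from a parent gun, that fires a volley of projectiles from arrow components for one ammo.
; Shoot waits the fire delay, spawns projectiles with explosion effects and sound, and plays a timeline-driven recoil lerp on the mesh.
; It then updates the player character's ammo and calls itself, repeating while CanShoot sees fire wanted and no reload.
; An empty magazine triggers the character's reload.
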(event EventBeginPlay
  (bind _shotguntransform (Variables|Default|GetShotgunTransform))
  (|CallParentFunction)
  (bind _output_get (Variables|Default|SetMaxAmmo (Variables|Default|GetShotgunMaxAmmo)))
  (Variables|Default|SetAmmo _output_get)
  (Utilities|Array|AddUnique _shotguntransform (Variables|Default|GetArrow1))
  (Utilities|Array|AddUnique _shotguntransform (Variables|Default|GetArrow)))

(event Collision|EventActorBeginOverlap
  (params (OtherActor :type Actor%20Object%20Reference))
  (|CallParentFunction OtherActor) ; This node is disabled and will not be called.\nDrag off pins to build functionality.
)

(event EventTick
  (params (DeltaSeconds :type Float%20%28single-precision%29))
  (|CallParentFunction DeltaSeconds) ; This node is disabled and will not be called.\nDrag off pins to build functionality.
)

(event EventShoot
  (bind _ammo (Variables|Default|GetAmmo))
  (Utilities|CanShoot
    (:true
      (if (> (Variables|Default|GetAmmo) 0)
        (Variables|Default|SetIsShooting true)
        (Utilities|FlowControl|Delay (Variables|Default|GetFireRatio))
        (for _index (range 0 (Variables|Default|GetShotgunBullet))
          (Utilities|FlowControl|Sequence
            (:then_0
              (Game|SpawnActorfromClass "/Game/Blueprint/Projectile/BP_Projectile.BP_Projectile_C" (Transformation|GetWorldTransform (Utilities|Array|Get(acopy) (Variables|Default|GetShotgunTransform) _index)) "AlwaysSpawn" "MultiplyWithRoot" 0 0)
              (Effects|SpawnEmitterAttached "/Game/Unreal/StarterContent/Particles/P_Explosion.P_Explosion" (Variables|Default|GetArrow) "None" (.Location (Math|Transform|BreakTransform (Transformation|GetRelativeTransform (Utilities|Array|Get(acopy) (Variables|Default|GetShotgunTransform) _index)))) (.Rotation (Math|Transform|BreakTransform (Transformation|GetRelativeTransform (Utilities|Array|Get(acopy) (Variables|Default|GetShotgunTransform) _index)))) "0.200000,0.200000,0.200000")
              (Audio|PlaySoundatLocation "/Game/Unreal/StarterContent/Audio/Collapse_Cue.Collapse_Cue" (Transformation|GetWorldLocation (Variables|Default|GetArrow)) "0, 0, 0" 0.1 1.0 0.0 0 0 0 0))
            (:then_1
              (bind _newtrack_0 (Timeline|Timeline PlayFromStart)
                (:Update
                  (Transformation|SetRelativeTransform (Variables|Default|GetSkeletalMesh) (Math|Transform|Lerp(Transform) (Math|Transform|MakeTransform "-10.000000,0.000000,2.000000" "0.000000,180.000000,0.000000" "1.000000,1.000000,1.000000") (Variables|Default|GetRecoil%20Position) (* _newtrack_0 (Variables|Default|GetRecoil%20Intensity))) false false))))))
        (Math|Integer|DecrementInt _ammo
          (:%20%20
            (bind _asbp_character (Utilities|Casting|CastToBP_Character (Game|GetPlayerCharacter 0)))
            (Default|CallOnAmmoChanged _asbp_character _ammo)
            (CallFunction|Shoot)))
        (else
          (bind _asbp_character_2 (Utilities|Casting|CastToBP_Character (Game|GetPlayerCharacter 0)))
          (Default|Reload _asbp_character_2)
          (Variables|Default|SetIsShooting false))))
    (:false
      (Variables|Default|SetIsShooting false))))

(fn ConstructionScript
  (|CallParentFunction))