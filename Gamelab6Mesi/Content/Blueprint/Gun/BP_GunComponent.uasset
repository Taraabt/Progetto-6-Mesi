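; Gun component that manages a set of gun actors for the player character and tracks the active one.
; Init validates and stores the holster and gun array, binds SwapGun to BP_Character's swap event, then selects the first gun, printing an error on invalid input.
; SwapGun switches guns by toggling actor visibility, updates CurrentGun and reports its ammo to the player pawn on each loop iteration.
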(event Custom|SwapGun
  (params (GunIndex :type Integer))
  (Utilities|FlowControl|Sequence
    (:then_0
      (for (_array_element _array_index) (Variables|Default|GetGun)
        (if (== GunIndex _array_index)
          (Rendering|SetActorHiddenInGame _array_element false)
          (Variables|Default|SetCurrentGun _array_element)
          (else
            (Rendering|SetActorHiddenInGame _array_element true)))
        (bind _asbp_character (Utilities|Casting|CastToBP_Character (Game|Player|GetPlayerPawn 0)))
        (Default|CallOnAmmoChanged _asbp_character (Variables|/Game/Blueprint/Gun/BP_Gun.BP_Gun_C|GetAmmo (Variables|Default|GetCurrentGun)))))))

(event Custom|Init
  (params (Gun :type Array%20of%20BP%20Gun%20Object%20References) (WepaonHoldster :type Camera%20Component%20Object%20Reference))
  (Utilities|IsValid WepaonHoldster
    (:Is%20Valid
      (if (Utilities|Array|IsEmpty Gun)
        (Development|PrintString (Utilities|String|Append (Utilities|GetDisplayName self) "failed init") :!label _label)
        (else
          (Variables|Default|SetWeaponHoldster WepaonHoldster)
          (Variables|Default|SetGun Gun)
          (bind _asbp_character (Utilities|Casting|CastToBP_Character (Game|Player|GetPlayerPawn 0)))
          (EventDispatchers|BindEventtoSwapGun _asbp_character (EventDispatchers|CreateEvent :!event Custom|SwapGun))
          (CallFunction|SwapGun))))
    (:Is%20Not%20Valid
      (goto _label))))

(event EventTick
  (params (DeltaSeconds :type Float%20%28single-precision%29)))

(event EventBeginPlay)