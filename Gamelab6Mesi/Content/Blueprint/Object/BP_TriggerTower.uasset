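; BP_TriggerTower is a trigger object that starts a losing countdown when BP_Character enters its sphere.
; The countdown spawns pool index 0 from its enemy pooler, initialized on BeginPlay, then waits CountDown seconds.
; When the delay ends, it pauses the game, switches to UI-only input with a visible cursor and shows WB_LoseScreen.
; The overlap checks IsCountDownStart, but this graph never sets it.
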(event OnComponentBeginOverlap(Sphere)
  (params (OverlappedComponent :type Primitive%20Component%20Object%20Reference) (OtherActor :type Actor%20Object%20Reference) (OtherComp :type Primitive%20Component%20Object%20Reference) (OtherBodyIndex :type Integer) (bFromSweep :type Boolean) (SweepResult :type Hit%20Result%20Structure%20%28by%20ref%29))
  (Utilities|Casting|CastToBP_Character OtherActor)
  (if (not (Variables|Default|GetIsCountDownStart))
    (CallFunction|StartCountDown)))

(event Custom|StartCountDown
  (bind _returnvalue (Game|GetPlayerController 0))
  (Default|SpawnfromPool (Variables|Default|GetBP_EnemyPoolerComponent))
  (Utilities|FlowControl|Delay (Variables|Default|GetCountDown))
  (Input|SetInputModeUIOnly _returnvalue 0 "DoNotLock" false)
  (Variables|/Script/Engine.PlayerController|SetbShowMouseCursor _returnvalue true)
  (Game|SetGamePaused true)
  (bind _returnvalue_2 (Game|ConstructObjectfromClass "/Game/widget/Lose/WB_LoseScreen.WB_LoseScreen_C"))
  (UserInterface|Viewport|AddtoViewport _returnvalue_2 0))

(event EventBeginPlay
  (Default|InitializePool (Variables|Default|GetBP_EnemyPoolerComponent)))

(event EventTick
  (params (DeltaSeconds :type Float%20%28single-precision%29)))

(fn ConstructionScript)