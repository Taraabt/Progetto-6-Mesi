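; BP_Wall is a breakable wall that gates progression between enemy spawners.
; When it takes BP_StunDamage, it checks that the Pooler's current spawner has an EnemyToKill count of zero.
; It then advances the Pooler index and either spawns the next spawner's enemy or, if none is valid, calls CanArenaSpawn.
; The wall destroys itself in both cases.
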(event Collision|EventActorBeginOverlap
  (params (OtherActor :type Actor%20Object%20Reference)))

(event EventTick
  (params (DeltaSeconds :type Float%20%28single-precision%29)))

(event Game|Damage|EventAnyDamage
  (params (Damage :type Float%20%28single-precision%29) (DamageType :type Damage%20Type%20Object%20Reference) (InstigatedBy :type Controller%20Object%20Reference) (DamageCauser :type Actor%20Object%20Reference))
  (bind _pooler (Variables|Default|GetPooler))
  (if (Class|GameplayStatics|ObjectIsA DamageType "/Game/Blueprint/Projectile/BP_StunDamage.BP_StunDamage_C")
    (if (== (Variables|/Game/Blueprint/Enemy/BP_EnemySpawner.BP_EnemySpawner_C|GetEnemyToKill (Utilities|Array|Get(acopy) (Variables|/Game/Blueprint/ObjectPool/BP_EnemyPooler.BP_EnemyPooler_C|GetSpawner _pooler) (Variables|/Game/Blueprint/ObjectPool/BP_EnemyPooler.BP_EnemyPooler_C|GetIndex _pooler))) 0)
      (bind _result (Math|Integer|IncrementInt (Variables|/Game/Blueprint/ObjectPool/BP_EnemyPooler.BP_EnemyPooler_C|GetIndex _pooler))
        (:%20%20
          (Variables|/Game/Blueprint/ObjectPool/BP_EnemyPooler.BP_EnemyPooler_C|SetIndex _pooler _result)
          (Utilities|IsValid (Utilities|Array|Get(acopy) (Variables|/Game/Blueprint/ObjectPool/BP_EnemyPooler.BP_EnemyPooler_C|GetSpawner _pooler) (Variables|/Game/Blueprint/ObjectPool/BP_EnemyPooler.BP_EnemyPooler_C|GetIndex _pooler))
            (:Is%20Valid
              (Default|SpawnEnemy (Utilities|Array|Get(acopy) (Variables|/Game/Blueprint/ObjectPool/BP_EnemyPooler.BP_EnemyPooler_C|GetSpawner _pooler) (Variables|/Game/Blueprint/ObjectPool/BP_EnemyPooler.BP_EnemyPooler_C|GetIndex _pooler)))
              (Actor|DestroyActor))
            (:Is%20Not%20Valid
              (Default|CallCanArenaSpawn)
              (Actor|DestroyActor))))))))

(fn ConstructionScript)

(fn BPWallAutoGenFunc)