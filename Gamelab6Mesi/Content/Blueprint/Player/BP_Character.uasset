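; First-person player character with movement, jump, a cooldown-limited dash, automatic gun fire and health.
; Holding Shoot runs a self-calling delayed loop gated by the CanShoot macro, spawning projectiles with effects and timeline-driven recoil, and auto-reloading when empty.
; Dash launches along current velocity, or camera forward when stationary.
; Ammo and damage changes fire dispatchers; death only prints, and M applies debug self-damage.
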(event Custom|ShootingLoop
  (bind _projectile_spawn (Variables|Default|GetProjectile%20Spawn))
  (bind _returnvalue (Transformation|GetRelativeTransform _projectile_spawn))
  (bind (_location _rotation) (Math|Transform|BreakTransform _returnvalue))
  (Utilities|CanShoot
    (:true
      (if (> (Variables|PlayerStats|GetAmmo) 0)
        (Variables|Default|SetIsShooting true)
        (Utilities|FlowControl|Delay (Variables|PlayerStats|GetFireRatio))
        (bind _result (Math|Integer|DecrementInt (Variables|PlayerStats|GetAmmo))
          (:%20%20
            (Default|CallOnAmmoChanged _result)
            (Utilities|FlowControl|Sequence
              (:then_0
                (Game|SpawnActorfromClass "/Game/Blueprint/BP_Projectile.BP_Projectile_C" (Transformation|GetWorldTransform _projectile_spawn) "AlwaysSpawn" "MultiplyWithRoot" 0 0)
                (Effects|SpawnEmitterAttached "/Game/Unreal/StarterContent/Particles/P_Explosion.P_Explosion" (Variables|Default|GetSK_FPGun) "None" _location _rotation "0.200000,0.200000,0.200000")
                (Audio|PlaySoundatLocation "/Game/Unreal/StarterContent/Audio/Explosion_Cue.Explosion_Cue" _location "0, 0, 0" 1.0 1.0 0.0 0 0 0 0)
                (CallFunction|ShootingLoop))
              (:then_1
                (bind _newtrack_0 (Timeline|RecoilTimeline PlayFromStart)
                  (:Update
                    (Pawn|Input|AddControllerPitchInput (* (* _newtrack_0 (Variables|Default|GetRecoilIntensity)) -0.3))
                    (Transformation|SetRelativeTransform (Variables|Default|GetSK_FPGun) (Math|Transform|Lerp(Transform) (Math|Transform|MakeTransform "-50.000000,20.000000,93.000000" "0, 0, 0" "1.000000,1.000000,1.000000") (Variables|Default|GetRecoilPosition) (* _newtrack_0 (Variables|Default|GetRecoilIntensity))) false false)))))))
        (else
          (CallFunction|Reload)
          (Variables|Default|SetIsShooting false))))
    (:false
      (Variables|Default|SetIsShooting false))))

(event Custom|Reload
  (Variables|Default|SetIsReloading true)
  (Utilities|FlowControl|Delay (Variables|PlayerStats|GetReloadRate))
  (bind _output_get (Variables|PlayerStats|SetAmmo 30))
  (Default|CallOnAmmoChanged _output_get)
  (Variables|Default|SetIsReloading false)
  (if (Variables|Default|GetWantShoot)
    (CallFunction|ShootingLoop)))

(event EventTick
  (params (DeltaSeconds :type Float%20%28single-precision%29)))

(event Game|Damage|EventAnyDamage
  (params (Damage :type Float%20%28single-precision%29) (DamageType :type Damage%20Type%20Object%20Reference) (InstigatedBy :type Controller%20Object%20Reference) (DamageCauser :type Actor%20Object%20Reference))
  (Variables|PlayerStats|SetHealth (- (Variables|PlayerStats|GetHealth) Damage))
  (if (< (Variables|PlayerStats|GetHealth) 0.0)
    (Development|PrintString "dead")
    (else
      (Default|CallOnPlayerDamage (Variables|PlayerStats|GetHealth)))))

(event Input|ActionEvents|InputActionJump
  (params (Key :type Key%20Structure :default "None"))
  (:Pressed
    (Character|Jump)))

(event Input|ActionEvents|InputActionDash
  (params (Key :type Key%20Structure :default "None"))
  (bind _returnvalue (Transformation|GetVelocity))
  (bind _dashmultiplier (Variables|PlayerStats|GetDashMultiplier))
  (bind _camera (Variables|Default|GetCamera))
  (bind (_x _y) (Math|Vector|BreakVector _returnvalue))
  (bind _returnvalue_2 (Math|Vector|GetForwardVector _camera))
  (bind _returnvalue_3 (* _returnvalue 1e+01))
  (bind _returnvalue_4 (* _returnvalue_2 _dashmultiplier))
  (:Pressed
    (if (not (Variables|Default|GetIsDashing))
      (Variables|Default|SetIsDashing true)
      (if (Utilities|Operators|EqualEqual :A (Math|Vector2D|MakeVector2D _x _y) :ErrorTolerance 1.0)
        (Character|LaunchCharacter (Math|Vector|MakeVector (.x _returnvalue_4) (.y _returnvalue_4) 0.0) false false)
        (Utilities|FlowControl|Delay 1.0)
        (Variables|Default|SetIsDashing false)
        (else
          (Character|LaunchCharacter (Math|Vector|MakeVector (.x _returnvalue_3) (.y _returnvalue_3) 0.0) false false)
          (Utilities|FlowControl|Delay 1.0)
          (Variables|Default|SetIsDashing false))))))

(event Input|ActionEvents|InputActionShoot
  (params (Key :type Key%20Structure :default "None"))
  (:Pressed
    (Variables|Default|SetWantShoot true)
    (CallFunction|ShootingLoop))
  (:Released
    (Variables|Default|SetWantShoot false)))

(event Input|ActionEvents|InputActionReload
  (params (Key :type Key%20Structure :default "None"))
  (:Pressed
    (CallFunction|Reload)))

(event Input|AxisEvents|InputAxisTurnLeftRight
  (params (AxisValue :type Float%20%28single-precision%29))
  (Pawn|Input|AddControllerYawInput AxisValue))

(event Input|AxisEvents|InputAxisLookUpDown
  (params (AxisValue :type Float%20%28single-precision%29))
  (Pawn|Input|AddControllerPitchInput AxisValue))

(event Input|AxisEvents|InputAxisBackForward
  (params (AxisValue :type Float%20%28single-precision%29))
  (Pawn|Input|AddMovementInput (Math|Vector|GetForwardVector (Variables|Collision|GetCapsuleComponent)) AxisValue false))

(event Input|AxisEvents|InputAxisLeftRight
  (params (AxisValue :type Float%20%28single-precision%29))
  (Pawn|Input|AddMovementInput (Math|Vector|GetRightVector (Variables|Collision|GetCapsuleComponent)) AxisValue false))

(event Input|KeyboardEvents|M
  (params (Key :type Key%20Structure :default "None"))
  (:Pressed
    (Game|Damage|ApplyDamage self 1e+01 0 0)))

(fn ConstructionScript)