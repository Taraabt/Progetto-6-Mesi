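; BP_EnemyBase is an enemy Blueprint that loses health when hit and awards points when destroyed.
; Each hit on its Scorpion03 component decrements HP.
; When HP reaches exactly zero, it calls the OnUpdateScore dispatcher on BP_GameInstance with its Score plus Points, then destroys itself.
; Its own UpdateScore event is empty.
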(event OnComponentHit(Scorpion03)
  (params (HitComponent :type Primitive%20Component%20Object%20Reference) (OtherActor :type Actor%20Object%20Reference) (OtherComp :type Primitive%20Component%20Object%20Reference) (NormalImpulse :type Vector :default "0, 0, 0") (Hit :type Hit%20Result%20Structure%20%28by%20ref%29))
  (bind _result (Math|Float|DecrementFloat (Variables|Default|GetHP))
    (:%20%20
      (if (== _result 0.0)
        (bind _asbp_game_instance (Utilities|Casting|CastToBP_GameInstance (Game|GetGameInstance)))
        (Default|CallOnUpdateScore _asbp_game_instance (+ (stale Custom|UpdateScore Score) (Variables|Default|GetPoints)))
        (Actor|DestroyActor)))))

(event Custom|UpdateScore
  (params (Score :type Integer)))

(event EventBeginPlay)

(event Collision|EventActorBeginOverlap
  (params (OtherActor :type Actor%20Object%20Reference)))

(event EventTick
  (params (DeltaSeconds :type Float%20%28single-precision%29)))

(fn ConstructionScript)