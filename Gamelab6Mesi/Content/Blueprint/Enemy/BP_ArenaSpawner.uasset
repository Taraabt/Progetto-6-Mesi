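; BP_ArenaSpawner fills an arena with pooled enemies and registers with LastWall's CanArenaSpawn event on BeginPlay.
; SpawnEnemy calls itself recursively until Index reaches the first NumberOfEnemy entry.
; Each call asks the Pooler's BPEnemyPoolerComponent for one of two random pool indices, using random actor-relative SpawnPoint locations and a rotation aimed at the player character.
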(event Custom|SpawnEnemy
  (if (< (Variables|Default|GetIndex) (Utilities|Array|Get(acopy) (Variables|Default|GetNumberOfEnemy)))
    (bind _asbp_character (Utilities|Casting|CastToBP_Character (Game|GetPlayerCharacter 0)))
    (bind _result (Math|Integer|DecrementInt (Utilities|Array|Length (Variables|Default|GetSpawnPoint)))
      (:%20%20
        (Default|SpawnfromPool (Variables|/Game/Blueprint/ObjectPool/BP_EnemyPooler.BP_EnemyPooler_C|GetBP_EnemyPoolerComponent (Variables|Default|GetPooler)) (Math|Transform|MakeTransform (.location (Math|Conversions|ToTransform(Vector) (Math|Transform|TransformLocation (Transformation|GetActorTransform) (Utilities|Array|Get(acopy) (Variables|Default|GetSpawnPoint) (Math|Random|RandomIntegerinRange 0 _result))))) (Math|Rotator|FindLookatRotation (.location (Math|Conversions|ToTransform(Vector) (Math|Transform|TransformLocation (Transformation|GetActorTransform) (Utilities|Array|Get(acopy) (Variables|Default|GetSpawnPoint) (Math|Random|RandomIntegerinRange 0 _result))))) (.location (Transformation|GetActorTransform _asbp_character))) (.scale (Math|Conversions|ToTransform(Vector) (Math|Transform|TransformLocation (Transformation|GetActorTransform) (Utilities|Array|Get(acopy) (Variables|Default|GetSpawnPoint) (Math|Random|RandomIntegerinRange 0 _result)))))) (Math|Random|RandomIntegerinRange 0 1))
        (Math|Integer|IncrementInt (Variables|Default|GetIndex)
          (:%20%20
            (CallFunction|SpawnEnemy)))))))

(event EventBeginPlay
  (EventDispatchers|BindEventtoCanArenaSpawn (Variables|Default|GetLastWall) (EventDispatchers|CreateEvent :!event Custom|SpawnEnemy)))

(fn ConstructionScript)