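; BP_EnemyAI is a reusable enemy that chases the player and awards score on death.
; Pawn sensing triggers AI movement toward the player, calling an empty Attack event within attack range.
; Stun damage disables movement for a few seconds, while other damage reduces health.
; Health exactly at zero updates the game instance score, signals death and clears the in-use state, which resets health through SetInUse.
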(event OnSeePawn(PawnSensing)
  (params (Pawn :type Pawn%20Object%20Reference))
  (Variables|Default|SetIsSeeingPlayer true)
  (CallFunction|FollowPlayer))

(event Custom|FollowPlayer
  (bind _self self)
  (if (Variables|Default|GetIsSeeingPlayer)
    (if (Variables|Default|GetCanMove)
      (AI|AIMoveTo _self "0, 0, 0" (Game|GetPlayerCharacter 0) (Variables|Default|GetAttackRange) false
        (:OnSuccess
          (CallFunction|Attack)))
      (else
        (AI|AIMoveTo _self "0, 0, 0" _self 0.0 false)))))

(event Custom|Stun
  (Variables|Default|SetCanMove false)
  (Utilities|FlowControl|Delay 3.0)
  (Variables|Default|SetCanMove true))

(event Custom|Attack)

(event EventBeginPlay)

(event Collision|EventActorBeginOverlap
  (params (OtherActor :type Actor%20Object%20Reference)))

(event EventTick
  (params (DeltaSeconds :type Float%20%28single-precision%29)))

(event Game|Damage|EventAnyDamage
  (params (Damage :type Float%20%28single-precision%29) (DamageType :type Damage%20Type%20Object%20Reference) (InstigatedBy :type Controller%20Object%20Reference) (DamageCauser :type Actor%20Object%20Reference))
  (if (Class|GameplayStatics|ObjectIsA DamageType "/Game/Blueprint/Projectile/BP_StunDamage.BP_StunDamage_C")
    (CallFunction|Stun)
    (else
      (bind _output_get (Variables|Default|SetCurrentHp (- (Variables|Default|GetCurrentHp) Damage)))
      (if (== _output_get 0.0)
        (bind _asbp_game_instance (Utilities|Casting|CastToBP_GameInstance (Game|GetGameInstance)))
        (Default|CallOnUpdateScore _asbp_game_instance (+ 0 (Variables|Default|GetPoints)))
        (Default|CallOnDeath)
        (CallFunction|SetinUse false)))))

(event EventSetinUse
  (params (InUse :type Boolean))
  (Variables|Default|SetCurrentHp (Variables|Default|GetHp))
  (|CallParentFunction InUse))

(fn ConstructionScript)