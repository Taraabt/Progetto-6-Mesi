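; Enemy spawner actor that releases a set number of pooled enemies at random spawn points, each rotated toward the player character.
; On BeginPlay it sets the kill count and, if active, starts SpawnEnemy, which re-calls itself after a delay until the total is reached.
; A percentage roll picks between two pairs of pool indices before calling SpawnFromPool on the Pooler's component.
; Spawn points are relative to the actor's transform.
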(event Custom|SpawnEnemy
  (bind _pooler (Variables|Default|GetPooler))
  (bind _index (Variables|Default|GetIndex))
  (bind _bp_enemypoolercomponent (Variables|/Game/Blueprint/ObjectPool/BP_EnemyPooler.BP_EnemyPooler_C|GetBP_EnemyPoolerComponent _pooler))
  (Development|PrintString (Utilities|String|ToString(Integer) _index))
  (Variables|Default|SetActive true)
  (if (< _index (Variables|Default|GetTotalNumberOfEnemy))
    (Development|PrintString "test")
    (bind _result (Math|Integer|DecrementInt (Utilities|Array|Length (Variables|Default|GetSpawnPoint)))
      (:%20%20
        (bind _asbp_character (Utilities|Casting|CastToBP_Character (Game|Player|GetPlayerPawn 0)))
        (if (>= (Math|Random|RandomFloatinRange 0.0 1e+02) (Variables|Default|GetPerc))
          (Default|SpawnfromPool _bp_enemypoolercomponent (Math|Transform|MakeTransform (.location (Math|Conversions|ToTransform(Vector) (Math|Transform|TransformLocation (Transformation|GetActorTransform) (Utilities|Array|Get(acopy) (Variables|Default|GetSpawnPoint) (Math|Random|RandomIntegerinRange 0 _result))))) (Math|Rotator|FindLookatRotation (.location (Math|Conversions|ToTransform(Vector) (Math|Transform|TransformLocation (Transformation|GetActorTransform) (Utilities|Array|Get(acopy) (Variables|Default|GetSpawnPoint) (Math|Random|RandomIntegerinRange 0 _result))))) (.location (Transformation|GetActorTransform _asbp_character))) (.scale (Math|Conversions|ToTransform(Vector) (Math|Transform|TransformLocation (Transformation|GetActorTransform) (Utilities|Array|Get(acopy) (Variables|Default|GetSpawnPoint) (Math|Random|RandomIntegerinRange 0 _result)))))) (Math|Random|RandomIntegerinRange 0 1))
          (else
            (Default|SpawnfromPool _bp_enemypoolercomponent (Math|Transform|MakeTransform (.location (Math|Conversions|ToTransform(Vector) (Math|Transform|TransformLocation (Transformation|GetActorTransform) (Utilities|Array|Get(acopy) (Variables|Default|GetSpawnPoint) (Math|Random|RandomIntegerinRange 0 _result))))) (Math|Rotator|FindLookatRotation (.location (Math|Conversions|ToTransform(Vector) (Math|Transform|TransformLocation (Transformation|GetActorTransform) (Utilities|Array|Get(acopy) (Variables|Default|GetSpawnPoint) (Math|Random|RandomIntegerinRange 0 _result))))) (.location (Transformation|GetActorTransform _asbp_character))) (.scale (Math|Conversions|ToTransform(Vector) (Math|Transform|TransformLocation (Transformation|GetActorTransform) (Utilities|Array|Get(acopy) (Variables|Default|GetSpawnPoint) (Math|Random|RandomIntegerinRange 0 _result)))))) (Math|Random|RandomIntegerinRange 2 3))))
        (Utilities|FlowControl|Delay (Variables|Default|GetSpawnDelay))
        (Math|Integer|IncrementInt (Variables|Default|GetIndex)
          (:%20%20
            (CallFunction|SpawnEnemy)))))))

(event EventBeginPlay
  (Utilities|FlowControl|Delay 1e-05)
  (Variables|Default|SetEnemyToKill (Variables|Default|GetTotalNumberOfEnemy))
  (if (Variables|Default|GetActive)
    (CallFunction|SpawnEnemy)))

(event Collision|EventActorBeginOverlap
  (params (OtherActor :type Actor%20Object%20Reference)))

(event EventTick
  (params (DeltaSeconds :type Float%20%28single-precision%29)))

(fn ConstructionScript)