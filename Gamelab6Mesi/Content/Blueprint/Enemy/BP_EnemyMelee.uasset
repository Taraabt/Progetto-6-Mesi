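; Melee enemy Blueprint that overrides its parent's Attack event to damage the player.
; After the parent logic, it plays a sped-up melee montage on the mesh.
; When the montage completes, it applies damage directly to player 0's character, with no hit or range check in this graph.
; It then waits AttackRatio before clearing IsAttacking.
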(event EventAttack
  (|CallParentFunction)
  (Animation|Montage|PlayMontage (Variables|Character|GetMesh) "/Game/Model/Model_animated/AM_AttackMelee.AM_AttackMelee" 5.0
    (:OnCompleted
      (Game|Damage|ApplyDamage (Game|GetPlayerCharacter 0) (Variables|Default|GetDamage) 0 0 "/Game/Blueprint/Projectile/BP_EnemyDamage.BP_EnemyDamage_C")
      (Utilities|FlowControl|Delay (Variables|Default|GetAttackRatio))
      (Variables|Default|SetIsAttacking false))))

(fn ConstructionScript
  (|CallParentFunction))