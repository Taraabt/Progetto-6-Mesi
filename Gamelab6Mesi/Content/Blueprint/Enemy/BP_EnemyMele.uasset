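; Melee enemy Blueprint that overrides the Attack event of its parent to damage the player.
; It calls the parent attack, waits for AttackRatio, then applies Damage to player character 0 with the BP_EnemyDamage type and clears IsAttacking.
; The branch after the delay is always true, so the hit lands without a range or overlap check in this Blueprint.
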(event EventBeginPlay
  (|CallParentFunction) ; This node is disabled and will not be called.\nDrag off pins to build functionality.
)

(event Collision|EventActorBeginOverlap
  (params (OtherActor :type Actor%20Object%20Reference))
  (|CallParentFunction OtherActor) ; This node is disabled and will not be called.\nDrag off pins to build functionality.
)

(event EventTick
  (params (DeltaSeconds :type Float%20%28single-precision%29))
  (|CallParentFunction DeltaSeconds) ; This node is disabled and will not be called.\nDrag off pins to build functionality.
)

(event EventAttack
  (|CallParentFunction)
  (Utilities|FlowControl|Delay (Variables|Default|GetAttackRatio))
  (if true
    (Game|Damage|ApplyDamage (Game|GetPlayerCharacter 0) (Variables|Default|GetDamage) 0 0 "/Game/Blueprint/Projectile/BP_EnemyDamage.BP_EnemyDamage_C")
    (Variables|Default|SetIsAttacking false)))

(fn ConstructionScript
  (|CallParentFunction))