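; BP_EnemySpawner is an enemy spawner that releases a set number of pooled enemies over time.
; It starts on BeginPlay if Active, or whenever SpawnEnemy is called, and initializes EnemyToKill to the total.
; SpawnEnemy pulls one of two random pool indices from the Pooler's component at a random actor-relative SpawnPoint, rotated toward the player.
; It re-calls itself after SpawnDelay until the total is reached, printing the count each call.
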(event Custom|SpawnEnemy
  (bind _index (Variables|Default|GetIndex))
  (Development|PrintString (Utilities|String|ToString(Integer) _index))
  (Variables|Default|SetActive true)
  (if (< _index (Variables|Default|GetTotalNumberOfEnemy))
    (bind _result (Math|Integer|DecrementInt (Utilities|Array|Length (Variables|Default|GetSpawnPoint)))
      (:%20%20
        (bind _asbp_character (Utilities|Casting|CastToBP_Character (Game|Player|GetPlayerPawn 0)))
        (Default|SpawnfromPool (Variables|/Game/Blueprint/ObjectPool/BP_EnemyPooler.BP_EnemyPooler_C|GetBP_EnemyPoolerComponent (Variables|Default|GetPooler)) (Math|Transform|MakeTransform (.location (Math|Conversions|ToTransform(Vector) (Math|Transform|TransformLocation (Transformation|GetActorTransform) (Utilities|Array|Get(acopy) (Variables|Default|GetSpawnPoint) (Math|Random|RandomIntegerinRange 0 _result))))) (Math|Rotator|FindLookatRotation (.location (Math|Conversions|ToTransform(Vector) (Math|Transform|TransformLocation (Transformation|GetActorTransform) (Utilities|Array|Get(acopy) (Variables|Default|GetSpawnPoint) (Math|Random|RandomIntegerinRange 0 _result))))) (.location (Transformation|GetActorTransform _asbp_character))) (.scale (Math|Conversions|ToTransform(Vector) (Math|Transform|TransformLocation (Transformation|GetActorTransform) (Utilities|Array|Get(acopy) (Variables|Default|GetSpawnPoint) (Math|Random|RandomIntegerinRange 0 _result)))))) (Math|Random|RandomIntegerinRange 0 1))
        (Math|Integer|IncrementInt (Variables|Default|GetIndex)
          (:%20%20
            (Utilities|FlowControl|Delay (Variables|Default|GetSpawnDelay))
            (CallFunction|SpawnEnemy)))))))

(event EventBeginPlay
  (Variables|Default|SetEnemyToKill (Variables|Default|GetTotalNumberOfEnemy))
  (if (Variables|Default|GetActive)
    (CallFunction|SpawnEnemy)))

(event Collision|EventActorBeginOverlap
  (params (OtherActor :type Actor%20Object%20Reference)))

(event EventTick
  (params (DeltaSeconds :type Float%20%28single-precision%29)))

(fn ConstructionScript)